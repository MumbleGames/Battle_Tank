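; Projectile Blueprint that supplies sound and camera feedback for firing and exploding.
; The Exploding event plays an explosion sound at the projectile's location.
; The Firing event plays a blast sound there, then, if the instigator's controller is a PlayerController_BP, plays a world camera shake centered on that player's camera location.
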(event `self.Exploding`
  (`GameplayStatics.PlaySoundAtLocation` "/Game/Sound/explosion.explosion" (`self.K2_GetActorLocation`)))

(event `self.Firing`
  (bind _returnvalue (`self.GetInstigatorController`))
  (`GameplayStatics.PlaySoundAtLocation` "/Game/Sound/Blast.Blast" (`self.K2_GetActorLocation`))
  (bind _asplayer_controller_bp (cast `/Game/Blueprints/PlayerController_BP` _returnvalue))
  (if (`KismetMathLibrary.ClassIsChildOf` (`GameplayStatics.GetObjectClass` _returnvalue) "/Game/Blueprints/PlayerController_BP.PlayerController_BP_C")
    (`GameplayStatics.PlayWorldCameraShake` "/Game/Blueprints/MyShake.MyShake_C" (`PlayerCameraManager.GetCameraLocation` (`PlayerController.PlayerCameraManager` _asplayer_controller_bp)) 0.0 500.0)))

(fn `UserConstructionScript`)